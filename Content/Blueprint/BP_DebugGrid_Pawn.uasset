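; BP_DebugGrid_Pawn is a debug pawn that wanders randomly across a BP_DebugGrid_Map to exercise grid movement.
; After a short startup delay, it sends its AI controller to a random cell in a ten-by-ten range via AITaskMoveToGrid.
; Whether the move succeeds or fails, it waits briefly and picks a new target, looping indefinitely.
; Each tick it prints its FireflyGridMovement component's current grid coordinate.
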(event `self.ReceiveBeginPlay`
  (bind _returnvalue (`KismetMathLibrary.RandomIntegerInRange` 0 9))
  (`KismetSystemLibrary.Delay` 1.0)
  (bind _returnvalue_2 (`GameplayStatics.GetActorOfClass` "/FireflyGridMap/Blueprint/BP_DebugGrid_Map.BP_DebugGrid_Map_C" :!label _label))
  (`/Engine/EditorBlueprintResources/StandardMacros.IsValid` _returnvalue_2
    (:`Is Valid`
      (`FireflyAITask_MoveToGrid.AITask_MoveToGrid` (`AIBlueprintHelperLibrary.GetAIController` self) (`FireflyGridMapBase.GetGridOfMap` _returnvalue_2 (make `FireflyGridCoordinate` _returnvalue _returnvalue))
        (:`OnRequestSucceeded`
          _)
        (:`OnRequestFailed`
          _))
      (`KismetSystemLibrary.Delay` 0.2)
      (goto _label))))

(event `self.ReceiveTick`
  (params (DeltaSeconds :type "Float (single-precision)"))
  (bind (_coordinate_x _coordinate_y) (break `FireflyGridCoordinate` (`FireflyGridBase.Coordinate` (`FireflyGridMovementComponent.CurrentGrid` (`self.FireflyGridMovement`)))))
  (`KismetSystemLibrary.PrintString` (`KismetStringLibrary.Concat_StrStr` (`KismetStringLibrary.Conv_IntToString` _coordinate_x) "///" (`KismetStringLibrary.Conv_IntToString` _coordinate_y)) true false (struct :`G` 0.66 :`B` 1.0 :`A` 1.0) 0.0))

(fn `UserConstructionScript`)